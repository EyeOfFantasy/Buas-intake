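; Level-finish trigger actor that times the player's run and shows the completion screen when its box is overlapped.
; BeginPlay adds the on-screen time widget, while Tick uses a one-second Delay as a gate to count seconds and minutes.
; Any overlap stops the timer, then once only opens the completed widget with UI-only input and a visible cursor.
; The construction script pins the actor to X zero with a fixed rotation.
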(event `self.ReceiveBeginPlay`
  ;[0 0.2431 1] Start time on screen and time system
  (set `self.Playing` true)
  (bind _returnvalue (`|CreateWidget` "/Game/Blueprints/WB_Time_On_Screen.WB_Time_On_Screen_C"))
  (`UserWidget.AddToViewport` _returnvalue 0))

(event `self.ReceiveTick`
  (params (DeltaSeconds :type "Float (single-precision)"))
  ;[1 0.09412 0.8] Add seconds and minutes
  (set `self.Deltatime` DeltaSeconds)
  (if (`self.Playing`)
    (`KismetSystemLibrary.Delay` 1.0)
    (set `self.Seconds` (+ (`self.Seconds`) 1))
    (if (> (`self.Seconds`) 59)
      (set `self.Seconds` 0)
      (set `self.Minutes` (+ (`self.Minutes`) 1)))))

(event `self.Box.OnComponentBeginOverlap`
  (params (OverlappedComponent :type "PrimitiveComponent Object Reference") (OtherActor :type "Actor Object Reference") (OtherComp :type "PrimitiveComponent Object Reference") (OtherBodyIndex :type Integer) (bFromSweep :type Boolean) (SweepResult :type "HitResult Structure (by ref)"))
  (bind _returnvalue (`GameplayStatics.GetPlayerController` 0))
  ;[0 0.2431 1] Here the win-screen is created, we tell it how long it took to complete. Then it's added to the screen and we make sure that the player can see their mouse and restart the level
  (set `self.Playing` false)
  (`/Engine/EditorBlueprintResources/StandardMacros.DoOnce` false
    (:`Completed`
      (bind _returnvalue_2 (`|CreateWidget` "/Game/Blueprints/WB_Level_Completed.WB_Level_Completed_C"))
      (`UserWidget.AddToViewport` _returnvalue_2 0)
      (`WidgetBlueprintLibrary.SetInputMode_UIOnlyEx` _returnvalue _returnvalue_2)
      (set `PlayerController.bShowMouseCursor` true _returnvalue))))

(fn `UserConstructionScript`
  (bind (_returnvalue_x _returnvalue_y _returnvalue_z) (`KismetMathLibrary.BreakVector` (`self.K2_GetActorLocation`)))
  (`self.K2_SetActorLocation` (`KismetMathLibrary.MakeVector` 0.0 _returnvalue_y _returnvalue_z) false true)
  (`self.K2_SetActorRotation` (struct :`Yaw` 90.0)))