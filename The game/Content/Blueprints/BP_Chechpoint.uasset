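; Checkpoint actor that the player activates with the C key while inside its trigger box, saving a spawn point.
; Box overlap toggles player input and the TurnOn flag, showing a C-button prompt until the checkpoint is activated.
; Pressing C writes the overlapping BP_ThirdPersonCharacter's transform to SpawnTransform in BP_ThirdPersonGameMode.
; Activation sets CheckpointOn, swaps the inactive model for the On model and hides the prompt.
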(event `self.ReceiveBeginPlay`
  ;[1 0.09412 0.8] Hide models as the level start
  (`SceneComponent.SetHiddenInGame` (`self.C_Button`) true false)
  (`SceneComponent.SetHiddenInGame` (`self.On`) true false))

(event `self.Box.OnComponentBeginOverlap`
  (params (OverlappedComponent :type "PrimitiveComponent Object Reference") (OtherActor :type "Actor Object Reference") (OtherComp :type "PrimitiveComponent Object Reference") (OtherBodyIndex :type Integer) (bFromSweep :type Boolean) (SweepResult :type "HitResult Structure (by ref)"))
  ;[0 0.2431 1] Option is turned on when in range and C button model is shown
  (`|ExecutionSequence`
    (:`then_0`
      (if (not (`self.Checkpoint on`))
        (`SceneComponent.SetHiddenInGame` (`self.C_Button`) false false)))
    (:`then_1`
      (`self.EnableInput` (`GameplayStatics.GetPlayerController` 0))
      (bind _asbp_third_person_character (cast `/Game/Blueprints/BP_ThirdPersonCharacter` OtherActor))
      (set `self.Turn on` true))))

(event `Key|C`
  (params (Key :type "Key Structure"))
  ;[1 0.09412 0.8] Turns on the check point and change models
  (:`Pressed`
    (if (`self.Turn on`)
      (bind _asbp_third_person_game_mode (cast `/Game/Blueprints/BP_ThirdPersonGameMode` (`GameplayStatics.GetGameMode`)))
      (set `/Game/Blueprints/BP_ThirdPersonGameMode.Spawn transform` (`self.GetTransform` (stale `self.Box.OnComponentBeginOverlap` _asbp_third_person_character)) _asbp_third_person_game_mode)
      (set `self.Checkpoint on` true)
      ;;[0 0.2431 1] Change model
      (`SceneComponent.SetHiddenInGame` (`self.On`) false false)
      (`SceneComponent.SetHiddenInGame` (`self.Checkpoint`) true false)
      (`SceneComponent.SetHiddenInGame` (`self.C_Button`) true false))))

(event `self.Box.OnComponentEndOverlap`
  (params (OverlappedComponent :type "PrimitiveComponent Object Reference") (OtherActor :type "Actor Object Reference") (OtherComp :type "PrimitiveComponent Object Reference") (OtherBodyIndex :type Integer))
  ;[0 0.2431 1] Option is turned off when out of range and hide C button model
  (`SceneComponent.SetHiddenInGame` (`self.C_Button`) true false)
  (`self.DisableInput` (`GameplayStatics.GetPlayerController` 0))
  (set `self.Turn on` false)
  (cast `/Game/Blueprints/BP_ThirdPersonCharacter` OtherActor))

(fn `UserConstructionScript`)